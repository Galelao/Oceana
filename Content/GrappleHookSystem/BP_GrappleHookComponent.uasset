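; Character component for a grappling hook that pulls the third-person player toward BP_GrapplehookTarget actors.
; While inactive, each Tick it highlights the visible nearby target closest to the camera's forward direction.
; AttemptGrapple spawns hook and cable, then a Tick-driven state machine launches the character up, pulls it in by velocity and flings it on arrival.
; Limited-use grapple count logic remains but is disconnected.
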(event `self.ReceiveBeginPlay`
  (bind _asbp_third_person_character (cast `/Game/ThirdPerson/Blueprints/Pawn/BP_ThirdPersonCharacter` (`self.GetOwner`)))
  (set `self.OwningCharacter` _asbp_third_person_character))

(event `self.ReceiveTick`
  (params (DeltaSeconds :type "Float (single-precision)"))
  (switch `/Game/GrappleHookSystem/EN_GrappleState` (`self.GrappleState`)
    (:`NewEnumerator0`
      (`self.Inactive`))
    (:`NewEnumerator1`
      (`self.Firing`)
      (`self.OnGrappleUsed`))
    (:`NewEnumerator2`
      (`self.NearTarget`))
    (:`NewEnumerator3`
      (`self.HitTarget`))))

(event `UpdateGrapplePickUps`
  ;[0.04688 0.04688 0.04688] Old Logic For Making Grapple Based on Amount
  ;;[1 1 1] Pickup GrappleHook Action and Call
)

(event `IncreaseGrapple`
  ;[0.04688 0.04688 0.04688] Old Logic For Making Grapple Based on Amount
  ;;[1 1 1] Logic for Increasing Grapple Amount
)

(event `IncreaseMaxGrapple`
  ;[0.04688 0.04688 0.04688] Old Logic For Making Grapple Based on Amount
  ;;[1 1 1] Logic for Increasing Max Grapple Amount
)

(event `Key|M`
  (params (Key :type "Key Structure"))
  ;[0.04688 0.04688 0.04688] Old Logic For Making Grapple Based on Amount
)

(fn `AttemptGrapple`
  (bind _owningcharacter (`self.OwningCharacter`))
  (bind _mesh (`Character.Mesh` _owningcharacter))
  (bind _returnvalue (`SkinnedMeshComponent.GetSocketBoneName` _mesh "RightHand"))
  (bind _returnvalue_location (`KismetMathLibrary.BreakTransform` (`SkinnedMeshComponent.GetBoneTransform` _mesh _returnvalue "RTS_World")))
  (switch `/Game/GrappleHookSystem/EN_GrappleState` (`self.GrappleState`)
    (:`NewEnumerator0`
      (bind _currenttarget (`self.CurrentTarget`)
        (:`then`
          (bind _returnvalue_2 (`|SpawnActorFromClass` "/Game/GrappleHookSystem/BP_Grapplehook.BP_Grapplehook_C" (`KismetMathLibrary.MakeTransform` (`self.OwnerLocation`)) "AlwaysSpawn" "MultiplyWithRoot" null _currenttarget 5000.0 null))
          (set `self.GrappleHook` _returnvalue_2)
          (bind _returnvalue_3 (`|SpawnActorFromClass` "/Game/GrappleHookSystem/BP_GRapplehookCable.BP_GRapplehookCable_C" (`KismetMathLibrary.MakeTransform` _returnvalue_location) "AdjustIfPossibleButAlwaysSpawn" "MultiplyWithRoot" null _owningcharacter))
          (bind _output_get (set `self.GrappleCable` _returnvalue_3))
          (`Actor.K2_AttachToComponent` _output_get null _returnvalue "SnapToTarget" "SnapToTarget" "SnapToTarget" true)
          (`CableComponent.SetAttachEndTo` (`CableActor.CableComponent` (`self.GrappleCable`)) (`self.GrappleHook`) "DefaultSceneRoot" "None")
          (`Actor.K2_SetActorRotation` (`self.OwningCharacter`) (`KismetMathLibrary.MakeRotFromZX` (0.0 0.0 1.0) (`self.OwnerToTarget`)) false)
          (set `self.GrappleState` "NewEnumerator1"))
        (:`else`)))))

(fn `FindBestTarget`
  (params (Targets :type "Array of Actor Object Reference"))
  (returns (Target :type "Actor Object Reference"))
  (locals (`CurrentTarget(Local)` :type "Actor Object Reference") (`CurrentAngel(Local)` :type "Float (double-precision)" :default 0.0) (`BestAngle(Local)` :type "Float (double-precision)") (`BestTarget(Local)` :type "Actor Object Reference"))
  (bind _owningcharacter (`self.OwningCharacter`))
  (for _array_element Targets
    (set `local.CurrentTarget(Local)` _array_element)
    (bind _outhit (`KismetSystemLibrary.LineTraceSingle` (`Actor.K2_GetActorLocation` (`self.OwningCharacter`)) (`Actor.K2_GetActorLocation` (`local.CurrentTarget(Local)`)) "TraceTypeQuery1" false (`|MakeArray` (`self.OwningCharacter`) :!type "Actor Object Reference") "None" true (struct :`R` 1.0 :`A` 1.0) (struct :`G` 1.0 :`A` 1.0) 0.5))
    (if (== (`.HitActor` (`GameplayStatics.BreakHitResult` _outhit)) (`local.CurrentTarget(Local)`))
      (`|ExecutionSequence`
        (:`then_0`
          ;[1 1 1] (Step 1) Calculate Angele to Target
          (set `local.CurrentAngel(Local)` (`KismetMathLibrary.DegAcos` (`KismetMathLibrary.Dot_VectorVector` (`KismetMathLibrary.Normal` (- (`Actor.K2_GetActorLocation` (`local.CurrentTarget(Local)`)) (`Actor.K2_GetActorLocation` _owningcharacter))) (`SceneComponent.GetForwardVector` (`/Game/ThirdPerson/Blueprints/Pawn/BP_ThirdPersonCharacter.FollowCamera` _owningcharacter))))))
        (:`then_1`
          ;[1 1 1] (Step 2) If the angle is less than current angle or there is no best target, make this teh next target
          (if (or (< (`local.CurrentAngel(Local)`) (`local.BestAngle(Local)`)) (not (`KismetSystemLibrary.IsValid` (`local.BestTarget(Local)`))))
            (set `local.BestTarget(Local)` (`local.CurrentTarget(Local)`))
            (set `local.BestAngle(Local)` (`local.CurrentAngel(Local)`)))))))
  (return (`local.BestTarget(Local)`)))

(fn `Firing`
  (if (< (`/Game/GrappleHookSystem/BP_Grapplehook.DistanceToTarget` (`self.GrappleHook`)) (`self.StartJumpDistance`))
    (`GameplayStatics.PlaySound2D` (`KismetArrayLibrary.Array_Random` (`self.GrappleHitSFXArray`)) 1.0 1.0 0.0 null null)
    (`Character.LaunchCharacter` (`self.OwningCharacter`) (0.0 0.0 500.0) true true)
    (set `self.GrappleState` "NewEnumerator2")))

(fn `HitTarget`
  (bind (_returnvalue_x _returnvalue_y _returnvalue_z) (`KismetMathLibrary.BreakVector` (* (`self.CharacterInitialDirection`) 25000.0)))
  (if (< (`Actor.GetDistanceTo` (`self.OwningCharacter`) (`self.CurrentTarget`)) (`self.EndJumpDistance`))
    (`Character.LaunchCharacter` (`self.OwningCharacter`) (`KismetMathLibrary.MakeVector` _returnvalue_x (- _returnvalue_y 0.0) (- _returnvalue_z 10000.0)) true true)
    (`self.SetCurrentTarget` null)
    (`Actor.K2_DestroyActor` (`self.GrappleCable`))
    (set `self.GrappleCable` null)
    (`Actor.K2_DestroyActor` (`self.GrappleHook`))
    (set `self.GrappleHook` null)
    (set `self.GrappleState` "NewEnumerator0")
    (else
      (set `MovementComponent.Velocity` (* (`self.OwnerToTarget`) (`self.CharacterGrappleSpeed`)) (`Pawn.GetMovementComponent` (`self.OwningCharacter`))))))

(fn `Inactive`
  (bind _outactors (`KismetSystemLibrary.SphereOverlapActors` (`Actor.K2_GetActorLocation` (`self.OwningCharacter`)) (`self.MaxGrappleDistance`) (`|MakeArray` "ObjectTypeQuery1" :!type "EObjectTypeQuery Enum") "/Game/GrappleHookSystem/BP_GrapplehookTarget.BP_GrapplehookTarget_C"))
  (bind _target (`self.FindBestTarget` _outactors))
  (`self.SetCurrentTarget` (cast `/Game/GrappleHookSystem/BP_GrapplehookTarget` _target :!pure true)))

(fn `NearTarget`
  (bind (_returnvalue_x _returnvalue_y _returnvalue_z) (`KismetMathLibrary.BreakVector` (`Actor.GetVelocity` (`self.OwningCharacter`))))
  (if (<= _returnvalue_z 0.0)
    (set `self.CharacterInitialDirection` (`self.OwnerToTarget`))
    (set `self.GrappleState` "NewEnumerator3")))

(fn `SetCurrentTarget`
  (params (NewTarget :type "/Game/GrappleHookSystem/BP_GrapplehookTarget Object Reference"))
  (if (!= NewTarget (`self.CurrentTarget`))
    (`|ExecutionSequence`
      (:`then_0`
        ;[1 1 1] Hide Old Target
        (bind _currenttarget (`self.CurrentTarget`)
          (:`then`
            (`/Game/GrappleHookSystem/BP_GrapplehookTarget.SetActive` _currenttarget false))
          (:`else`)))
      (:`then_1`
        ;[1 1 1] Set New Target
        (set `self.CurrentTarget` (`local.NewTarget`)))
      (:`then_2`
        ;[1 1 1] Show New Target
        (bind _currenttarget_2 (`self.CurrentTarget`)
          (:`then`
            (`/Game/GrappleHookSystem/BP_GrapplehookTarget.SetActive` _currenttarget_2 true))
          (:`else`))))))