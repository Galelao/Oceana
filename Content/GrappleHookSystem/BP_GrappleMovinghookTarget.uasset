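; Pawn for a moving grapple hook target that makes one move away from the player when play begins.
; BeginPlay issues an AI MoveTo toward a random reachable point around a spot offset along the direction from player to target, using a FloatingPawnMovement component.
; A successful move only triggers a short delay with nothing after it, so the movement does not repeat.
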(event `self.ReceiveBeginPlay`
  (bind _returnvalue (`self.K2_GetActorLocation`))
  (`|AIMoveTo` (`self.FloatingPawnMovement`) null (`NavigationSystemV1.K2_GetRandomReachablePointInRadius` (+ _returnvalue (* (`KismetMathLibrary.Normal` (- _returnvalue (`self.K2_GetActorLocation` (`GameplayStatics.GetPlayerCharacter` 0)))) 500.0)) 500.0 null null) null 200.0
    (:`OnSuccess`
      (`KismetSystemLibrary.Delay` 2.0))))

(fn `UserConstructionScript`
  (`parent.UserConstructionScript`))